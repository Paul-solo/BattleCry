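; Turret building that tracks pawns it sees through PawnSensing and fires at them, ignoring any pawn tagged "1".
; Each sighting yaws the actor toward the pawn, then aims Barrel and Arrow with pitch measured from the barrel.
; A Delay after aiming throttles firing, then an actor spawns at the Arrow transform with slight random pitch and yaw spread.
; The spawn node shows no actor class.
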(event OnSeePawn(PawnSensing)
  (params (Pawn :type Pawn%20Object%20Reference))
  (bind _returnvalue (Transformation|GetActorLocation Pawn))
  (bind _arrow (Variables|Default|GetArrow))
  (bind _barrel (Variables|Default|Getbarrel))
  (bind _turret_base (Variables|Default|Getturret_base))
  (bind _returnvalue_2 (Transformation|GetWorldLocation _turret_base))
  (bind _returnvalue_3 (Transformation|GetWorldTransform _arrow))
  (bind _returnvalue_4 (Math|Rotator|FindLookatRotation _returnvalue_2 _returnvalue))
  (if (not (Actor|ActorHasTag Pawn "1"))
    (Transformation|SetActorRotation (Math|Rotator|MakeRotator (.roll _returnvalue_4) 0.0 (.yaw _returnvalue_4)))
    (Transformation|SetWorldRotation _barrel (Math|Rotator|MakeRotator (.roll _returnvalue_4) (.pitch (Math|Rotator|FindLookatRotation (Transformation|GetWorldLocation _barrel) (Transformation|GetActorLocation Pawn))) (.yaw _returnvalue_4)) false false)
    (Utilities|FlowControl|Delay 1.0)
    (Game|SpawnActorfromClass "/Game/AI-1/bullet.bullet_C" (Math|Transform|MakeTransform (.location _returnvalue_3) (Math|Rotator|MakeRotator (.roll (.rotation _returnvalue_3)) (Math|Random|RandomFloatinRange (- (.pitch (.rotation _returnvalue_3)) 2.0) (+ (.pitch (.rotation _returnvalue_3)) 2.0)) (Math|Random|RandomFloatinRange (- (.yaw (.rotation _returnvalue_3)) 2.0) (+ (.yaw (.rotation _returnvalue_3)) 2.0))) (.scale _returnvalue_3)) "Undefined" "MultiplyWithRoot" 0 0)))

(event EventBeginPlay)

(event Collision|EventActorBeginOverlap
  (params (OtherActor :type Actor%20Object%20Reference)))

(event EventTick
  (params (DeltaSeconds :type Float%20%28single-precision%29)))

(fn ConstructionScript)