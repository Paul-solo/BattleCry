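; BP_Barraks is a barracks building actor that opens its UI when clicked.
; A click on either of its two static meshes creates a new UIBarraks widget, passes the building as its owning actor and adds it to the viewport.
; GetLocation exposes the world position of the Arrow component; nothing in this Blueprint calls it.
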(event OnClicked(StaticMesh1)
  (params (TouchedComponent :type Primitive%20Component%20Object%20Reference) (ButtonPressed :type Key%20Structure :default "None"))
  (bind _returnvalue (UserInterface|CreateWidget "/Game/buildings/UI-Barraks.UI-Barraks_C" 0 0))
  (Variables|/Game/buildings/UI-Barraks.UI-Barraks_C|SetOwningActor _returnvalue self)
  (UserInterface|Viewport|AddtoViewport _returnvalue 0))

(event OnClicked(StaticMesh)
  (params (TouchedComponent :type Primitive%20Component%20Object%20Reference) (ButtonPressed :type Key%20Structure :default "None"))
  (bind _returnvalue (UserInterface|CreateWidget "/Game/buildings/UI-Barraks.UI-Barraks_C" 0 0))
  (Variables|/Game/buildings/UI-Barraks.UI-Barraks_C|SetOwningActor _returnvalue self)
  (UserInterface|Viewport|AddtoViewport _returnvalue 0))

(event EventBeginPlay)

(event Collision|EventActorBeginOverlap
  (params (OtherActor :type Actor%20Object%20Reference)))

(event EventTick
  (params (DeltaSeconds :type Float%20%28single-precision%29)))

(fn ConstructionScript)

(fn GetLocation
  (return (Transformation|GetWorldLocation (Variables|Default|GetArrow))))