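; BP_RTSGameMode is an RTS game mode that advances enemy waves as groups of enemies are cleared.
; Four check events each test their own enemies-left counter, two feeding WaveA and two feeding WaveB.
; When a counter is zero, the event increments its wave variable and calls that group's own RespawnNextWave to trigger the next spawn.
; The counters are only read here, and the construction script is empty.
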(event Custom|check%20ennmy-1-11
  (if (== (Variables|Default|Getennemy%20left) 0)
    (Math|Integer|IncrementInt (Variables|Default|GetwaveA)
      (:%20%20
        (Default|CallRespawnNextWave-1-11)))))

(event Custom|Check%20ennemy-2-1
  (if (== (Variables|Default|GetEnnemy%20Left1) 0)
    (Math|Integer|IncrementInt (Variables|Default|GetwaveB)
      (:%20%20
        (Default|CallRespawnNextWave1)))))

(event Custom|Check-2-2
  (if (== (Variables|Default|GetEnnemy%20Left-2-2) 0)
    (Math|Integer|IncrementInt (Variables|Default|GetwaveB)
      (:%20%20
        (Default|CallRespawnNextWave1-2)))))

(event Custom|Check%20ennemy-1-12
  (if (== (Variables|Default|GetEnnemy%20Left-1-12) 0)
    (Math|Integer|IncrementInt (Variables|Default|GetwaveA)
      (:%20%20
        (Default|CallRespawnNextWave-1-12)))))

(fn ConstructionScript)